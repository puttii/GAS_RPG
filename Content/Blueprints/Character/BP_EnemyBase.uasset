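; BP_EnemyBase is the base enemy character Blueprint, handling spawn, facing and dissolve presentation.
; On BeginPlay a timeline drives the mesh's uniform scale as a spawn effect.
; UpdateFacingTarget feeds a location into the Motion Warping "FacingTarget"; a note says the input is not actually the projectile's location, despite its name.
; Separate body and weapon timelines animate the "Dissolve" parameter on supplied dynamic material instances.
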(event EventBeginPlay
  (bind _新建轨道_0 (Timeline|SpawnTimeline Play)
    (:Update
      (Transformation|SetRelativeScale3D (Variables|Character|GetMesh) (Math|Vector|MakeVector _新建轨道_0 _新建轨道_0 _新建轨道_0)))))

(event Collision|EventActorBeginOverlap
  (params (OtherActor :type Actor%20Object%20Reference)))

(event EventTick
  (params (DeltaSeconds :type Float%20%28single-precision%29)))

(event EventStartDissolveTimeline
  (params (DynamicInstance :type Material%20Instance%20Dynamic%20Object%20Reference))
  (bind _dissolvetrack (Timeline|DissolveTimeline Play)
    (:Update
      (Rendering|Material|SetScalarParameterValue DynamicInstance "Dissolve" _dissolvetrack :!class /Script/Engine.MaterialInstanceDynamic))))

(event EventStartWeaponDissolveTimeline
  (params (DynamicInstance :type Material%20Instance%20Dynamic%20Object%20Reference))
  (bind _weapondissolvetrack (Timeline|WeaponDissolveTimeline Play)
    (:Update
      (Rendering|Material|SetScalarParameterValue DynamicInstance "Dissolve" _weapondissolvetrack :!class /Script/Engine.MaterialInstanceDynamic))))

(event EventUpdateFacingTarget
  (params (ProjectileTargetLocation :type Vector%20%28by%20ref%29 :default "0, 0, 0"))
  ;[0.15 0.15 0.15 0.5] 这里输入不是projectile的location，懒得在代码里改了
  (Class|MotionWarpingComponent|AddorUpdateWarpTargetfromLocation (Variables|Default|GetMotionWarping) "FacingTarget" ProjectileTargetLocation))

(fn ConstructionScript)